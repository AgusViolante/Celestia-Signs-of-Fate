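; Behavior Tree task that picks the next target point for a BP_EnemyBase enemy to move to.
; It writes the location of the current TargetPoint entry to the BBTargetPoint blackboard key, then finishes successfully.
; Despite its name, the RandomTarget index steps through the array in order and wraps to zero.
; The task does no movement itself, as its AIMoveTo node is unconnected, and a failed cast never finishes it.
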(event `self.ReceiveExecuteAI`
  (params (OwnerController :type "AIController Object Reference") (ControlledPawn :type "Pawn Object Reference"))
  (bind _asbp_enemy_base (cast `/Game/Blueprints/IAEnemy/BP_EnemyBase` ControlledPawn))
  (bind _targetpoint (`/Game/Blueprints/IAEnemy/BP_EnemyBase.TargetPoint` _asbp_enemy_base))
  (`BTFunctionLibrary.SetBlackboardValueAsVector` (`self.BB_TargetPoint`) (`Actor.K2_GetActorLocation` (`|GetArrayItem` _targetpoint (`self.RandomTarget`))))
  (if (>= (`self.RandomTarget`) (- (`KismetArrayLibrary.Array_Length` _targetpoint) 1))
    (set `self.RandomTarget` 0)
    (else
      (bind _result (`/Engine/EditorBlueprintResources/StandardMacros.IncrementInt` (`self.RandomTarget`))
        (:`  `
          (set `self.RandomTarget` _result)))))
  (`self.FinishExecute` true))